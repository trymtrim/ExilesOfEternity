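; Base Blueprint for battle royale characters, handling spellcasting, death, respawn UI, HUD and material swaps through server, client and broadcast events.
; UseSpellBP casts instant spells or starts a client-side aiming projection, which ActivateProjectionSpellBP resolves into a spawned spell actor.
; Blink finds ground by vertical traces and backs out of obstructions, while Meditate applies per-tick damage to self until expiry, movement or cancellation.
; Animation, death and reset broadcasts are empty here; debug events grant spells and experience.
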(event OnComponentHit(CapsuleComponent)
  (params (HitComponent :type Primitive%20Component%20Object%20Reference) (OtherActor :type Actor%20Object%20Reference) (OtherComp :type Primitive%20Component%20Object%20Reference) (NormalImpulse :type Vector :default "0, 0, 0") (Hit :type Hit%20Result%20Structure%20%28by%20ref%29))
  ;[1 1 1] Death in water
  (if (Networking|IsServer)
    (if (Utilities|IsValid OtherActor)
      (if (Actor|ActorHasTag OtherActor "Death")
        (Class|CharacterBase|Die)))))

(event Custom|BroadcastDeath
  ;[1 1 1] Character death
)

(event Custom|ClientDeath
  ;[1 1 1] Character death
  (Default|ToggleCrosshair (Variables|Default|GetBaseUI) false))

(event Custom|ServerAddSpells
  ;[1 1 1] Debug
  (Class|CharacterBase|AddSpell "FLAMESTRIKE")
  (Class|CharacterBase|AddSpell "CYCLONE")
  (Class|CharacterBase|AddSpell "BLINK")
  (Class|CharacterBase|AddSpell "CONTAINMENT_FENCE")
  (Class|CharacterBase|AddSpell "SHIELD")
  (Class|CharacterBase|AddSpell "MEDITATE"))

(event Custom|ServerStartGame
  ;[1 1 1] Debug
  (bind _asbattle_royale_game_mode (Utilities|Casting|CastToBattleRoyaleGameMode (Game|GetGameMode)))
  (Class|BattleRoyaleGameMode|PlaytestStartGame _asbattle_royale_game_mode (Pawn|GetController)))

(event Custom|ServerDie
  ;[1 1 1] Debug
  (bind _ascharacter_base (Utilities|Casting|CastToCharacterBase (Pawn|GetControlledPawn (Pawn|GetController))))
  (Class|CharacterBase|Die _ascharacter_base))

(event Custom|ServerGainExperience
  ;[1 1 1] Debug
  (bind _asbattle_royale_player_state (Utilities|Casting|CastToBattleRoyalePlayerState (Variables|Default|GetPlayerState)))
  (Class|BattleRoyalePlayerState|GainExperience _asbattle_royale_player_state 80))

(event Custom|ClientAddSpell
  (params (Spell :type Spells%20Enum :default "EMPTY"))
  ;[1 1 1] Add spell
  (if (Utilities|Enum|Equal(Enum) Spell "EMPTY")
    (bind _returnvalue (UserInterface|CreateWidget "/Game/UI/Spells/EmptySpell_Icon.EmptySpell_Icon_C"))
    (Class|UIHandler|AddSpelltoPanel (Variables|Default|Get_uiHandler) Spell _returnvalue)
    (else
      (bind _returnvalue_2 (UserInterface|CreateWidget "/Game/UI/Spells/Spell_Icon.Spell_Icon_C"))
      (Default|SetSpell _returnvalue_2 Spell)
      (Class|UIHandler|AddSpelltoPanel (Variables|Default|Get_uiHandler) Spell _returnvalue_2))))

(event Custom|ServerResetCooldowns
  ;[1 1 1] Debug
  (Class|CharacterBase|ResetCooldowns))

(event Custom|BroadcastResetCharacter
  ;[1 1 1] Reset character
)

(event Custom|BroadcastChangeMaterial
  (params (Material :type Material%20Object%20Reference))
  ;[1 1 1] Change material
  (for (_ _array_index) (Rendering|Material|GetMaterials (Variables|Character|GetMesh))
    (if (== (Utilities|GetClass self) "/Game/Blueprints/Characters/Serath_BP.Serath_BP_C")
      (if (not (or (== _array_index 12) (== _array_index 13)))
        (Rendering|Material|SetMaterial (Variables|Character|GetMesh) _array_index Material :!label _label))
      (else
        (goto _label)))))

(event Custom|ClientResetCharacter
  ;[1 1 1] Reset character
  (Default|ToggleCrosshair (Variables|Default|GetBaseUI) true))

(event Custom|BroadcastResetMaterial
  ;[1 1 1] Reset material
  (for (_ _array_index) (Variables|Default|GetCharacterMaterials)
    (Rendering|Material|SetMaterial (Variables|Character|GetMesh) _array_index 0)))

(event Custom|ChangeMaterial
  (params (Material :type Material%20Object%20Reference))
  ;[1 1 1] Change material
  (CallFunction|BroadcastChangeMaterial Material))

(event Custom|ResetMaterial
  ;[1 1 1] Reset material
  (CallFunction|BroadcastResetMaterial))

(event EventBeginPlay
  (Variables|Default|SetCharacterMaterials (Rendering|Material|GetMaterials (Variables|Character|GetMesh)))
  ;[1 1 1] Initialize character UI
  (if (Pawn|IsLocallyControlled)
    (bind _returnvalue (UserInterface|CreateWidget "/Game/UI/Player/Base_UI.Base_UI_C"))
    (UserInterface|Viewport|AddtoViewport _returnvalue 0)
    (Variables|Default|SetBaseUI _returnvalue)
    (Components|DestroyComponent (Variables|Default|GetHealthUI))
    (else
      (bind _ashealth_bar_ui (Utilities|Casting|CastToHealthBar_UI (UserInterface|GetUserWidgetObject (Variables|Default|GetHealthUI))))
      (Variables|/Game/UI/Player/HealthBar_UI.HealthBar_UI_C|SetCharacterController _ashealth_bar_ui self))))

(event EventTick
  (params (DeltaSeconds :type Float%20%28single-precision%29))
  (bind _baseui (Variables|Default|GetBaseUI))
  (if (Networking|IsServer)
    (CallFunction|CheckChannelingMeditate)
    (elif (Pawn|IsLocallyControlled)
      ;[1 1 1] Check for change in spell panel
      (bind _returnvalue (Class|UIHandler|GetSpellPositionChanged (Variables|Default|Get_uiHandler)))
      (if _returnvalue
        (Widget|RemovefromParent _baseui)
        (Utilities|FlowControl|Delay 0.0)
        (UserInterface|Viewport|AddtoViewport _baseui 0))
      (else
        (Transformation|SetWorldRotation (Variables|Default|GetHealthUI) (Math|Conversions|RotationFromXVector (- (Transformation|GetActorLocation (Game|GetPlayerCameraManager 0)) (Transformation|GetWorldLocation (Variables|Default|GetHealthUI)))) false false)))))

(event EventDieBP
  ;[1 1 1] Character death
  (CallFunction|ClientDeath)
  (CallFunction|BroadcastDeath))

(event EventAddSpellBP
  (params (spell :type Spells%20Enum :default "EMPTY"))
  ;[1 1 1] Add spell
  (CallFunction|ClientAddSpell spell))

(event EventServerInitializeCharacterBP
  ;[1 1 1] Initialize server specific elements after everything else is set up
  (bind _returnvalue (Game|GetCurrentLevelName true))
  (if (Utilities|Enum|Equal(Enum) _returnvalue "ArenaLevel")
    (Class|CharacterBase|AddSpell "FLAMESTRIKE")
    (Class|CharacterBase|AddSpell "CYCLONE")
    (Class|CharacterBase|AddSpell "BLINK")
    (Class|CharacterBase|AddSpell "CONTAINMENT_FENCE")
    (Class|CharacterBase|AddSpell "SHIELD")
    (Class|CharacterBase|AddSpell "MEDITATE")))

(event EventResetCharacterBP
  ;[1 1 1] Reset character
  (CallFunction|ClientResetCharacter)
  (CallFunction|BroadcastResetCharacter))

(event EventHandleRespawnBP
  ;[1 1 1] Character death
  (bind _returnvalue (UserInterface|CreateWidget "/Game/UI/BattleRoyale/BattleRoyaleRespawn_UI.BattleRoyaleRespawn_UI_C"))
  (UserInterface|Viewport|AddtoViewport _returnvalue 0)
  (bind _asbattle_royale_player_controller (Utilities|Casting|CastToBattleRoyalePlayerController (Pawn|GetController)))
  (Class|PlayerControllerBase|SetInputUIOnly _asbattle_royale_player_controller))

(event Input|KeyboardEvents|Enter
  (params (Key :type Key%20Structure))
  ;[1 1 1] Debug
)

(event Input|KeyboardEvents|Backspace
  (params (Key :type Key%20Structure))
  ;[1 1 1] Debug
)

(event Input|KeyboardEvents|0
  (params (Key :type Key%20Structure))
  ;[1 1 1] Debug
  (:Pressed
    (CallFunction|ServerAddSpells)))

(event Input|KeyboardEvents|Z
  (params (Key :type Key%20Structure))
  ;[1 1 1] Debug
)

(event Custom|BroadcastBlink
  (params (Location :type Vector))
  ;[1 1 1] Blink
  (Effects|SpawnEmitterAttached "/Game/FX/Spells/Blink/Blink_FX.Blink_FX" (Variables|Character|GetMesh) "None" "0.000000, 0,100.000000")
  (Audio|SpawnSoundAttached "/Game/Audio/Spells/Blink/Blink_OnUse.Blink_OnUse" (Variables|Default|GetAudio) "None" "0, 0, 0" "0, 0, 0" "KeepRelativeOffset" false 1.0 1.0 0.0 0 0)
  (Effects|SpawnEmitteratLocation "/Game/FX/AdvancedMagicFX13/Particles/P_ky_flash1.P_ky_flash1" Location))

(event Custom|CheckChannelingMeditate
  (bind _self self)
  ;[1 1 1] Meditate
  (if (Variables|Default|GetChannelingMeditate)
    (if (> (Math|Vector|VectorLength (Transformation|GetVelocity)) 0.1)
      (Variables|Default|SetChannelingMeditate false)
      (CallFunction|BroadcastCancelMediate)
      (else
        (bind _returnvalue (Class|SpellAttributes|GetDamage "MEDITATE" (stale EventUseSpellBP _returnvalue_9)))
        (Game|Damage|ApplyDamage _self (* (/ _returnvalue (stale EventUseSpellBP _returnvalue_10)) (Utilities|Time|GetWorldDeltaSeconds)) 0 _self)))))

(event Custom|BroadcastMeditate
  ;[1 1 1] Meditate
  (bind _returnvalue (Effects|SpawnEmitterAttached "/Game/FX/Spells/Meditate/Meditate_FX.Meditate_FX" (Variables|Character|GetMesh) "None"))
  (bind _returnvalue_2 (Audio|SpawnSoundAttached "/Game/Audio/Spells/Meditate/Meditate_OnUse.Meditate_OnUse" (Variables|Default|GetAudio) "None" "0, 0, 0" "0, 0, 0" "KeepRelativeOffset" true 1.0 1.0 0.0 0 0)))

(event Custom|BroadcastCancelMediate
  ;[1 1 1] Meditate
  (if (Utilities|IsValid (stale Custom|BroadcastMeditate _returnvalue))
    (Components|DestroyComponent (stale Custom|BroadcastMeditate _returnvalue))
    (CallFunction|CancelSpellAnimation)
    (if (Utilities|IsValid (stale Custom|BroadcastMeditate _returnvalue_2))
      (Audio|Components|Audio|FadeOut (stale Custom|BroadcastMeditate _returnvalue_2) 0.3 0.0 :!class /Script/Engine.AudioComponent)
      (Utilities|FlowControl|Delay 0.3)
      (Components|DestroyComponent (stale Custom|BroadcastMeditate _returnvalue_2)))))

(event Custom|CancelSpellAnimation)

(event Custom|BroadcastCyclone
  ;[1 1 1] Cyclone
  (Audio|SpawnSoundAttached "/Game/Audio/Spells/Cyclone/Cyclone_OnUse.Cyclone_OnUse" (Variables|Default|GetAudio) "None" "0, 0, 0" "0, 0, 0" "KeepRelativeOffset" false 1.0 1.0 0.0 0 0))

(event EventCancelCurrentSpellBP
  ;[1 1 1] Cancel current spell
  (if (Variables|Default|GetChannelingMeditate)
    (Variables|Default|SetChannelingMeditate false)
    (CallFunction|BroadcastCancelMediate)))

(event EventUseSpellBP
  (params (spell :type Spells%20Enum :default "EMPTY"))
  (bind _returnvalue (Transformation|GetActorLocation))
  (bind _returnvalue_2 (Transformation|GetActorForwardVector))
  (bind _bottomspellposition (Variables|Default|GetBottomSpellPosition))
  (bind _returnvalue_3 (* _returnvalue_2 1e+01))
  (bind _returnvalue_4 (- _returnvalue _returnvalue_3))
  (bind _returnvalue_5 (Class|SpellAttributes|GetType spell))
  (if (Utilities|Enum|Equal(Enum) _returnvalue_5 "PROJECTION")
    ;[1 1 1] Projection spells
    (CallFunction|ClientUseProjectingSpell spell :!label _label)
    (else
      (CallFunction|BroadcastPlayAnimation spell)
      (switch Utilities|FlowControl|Switch|SwitchonSpells spell
        (:FLAMESTRIKE
          (goto _label))
        (:SHIELD
          ;[1 1 1] Shield
          (Game|SpawnActorfromClass "/Game/Blueprints/Spells/ShieldSpell_BP.ShieldSpell_BP_C" (Math|Transform|MakeTransform (Transformation|GetActorLocation)) "Undefined" 0 self))
        (:BLINK
          ;[1 1 1] Blink
          (CallFunction|BroadcastBlink (Transformation|GetActorLocation))
          (bind _returnvalue_6 (Class|CharacterBase|GetSpellRank "BLINK"))
          (bind _returnvalue_7 (Class|SpellAttributes|GetRange "BLINK" _returnvalue_6))
          (bind _outhit (Collision|LineTraceByChannel (+ (* (Math|Conversions|ToVector(Float) _returnvalue_7) (Transformation|GetActorForwardVector)) (Transformation|GetActorLocation)) (+ (+ (* (Math|Conversions|ToVector(Float) _returnvalue_7) (Transformation|GetActorForwardVector)) (Transformation|GetActorLocation)) "0, 0,5000.000000") "TraceTypeQuery3" false 0 "None"))
          (if (Utilities|IsValid (.HitActor (Collision|BreakHitResult _outhit)))
            (if (not (Actor|ActorHasTag (.HitActor (Collision|BreakHitResult _outhit)) "Death"))
              (if (.bBlockingHit (Collision|BreakHitResult _outhit)) :!label _label_2
                (Transformation|SetActorLocation (+ (.Location (Collision|BreakHitResult _outhit)) "0, 0,100.000000") false false)
                (bind _returnvalue_8 (Collision|BoxTraceByChannel _returnvalue _returnvalue_4 "10.000000,10.000000,10.000000" "0, 0, 0" "TraceTypeQuery6" false 0 "None" :!label _label_3))
                (if _returnvalue_8
                  (Transformation|SetActorLocation _returnvalue_4 false false)
                  (goto _label_3))
                (else
                  (bind _outhit_2 (Collision|LineTraceByChannel (+ (* (Math|Conversions|ToVector(Float) _returnvalue_7) (Transformation|GetActorForwardVector)) (Transformation|GetActorLocation)) (- (+ (* (Math|Conversions|ToVector(Float) _returnvalue_7) (Transformation|GetActorForwardVector)) (Transformation|GetActorLocation)) "0, 0,5000.000000") "TraceTypeQuery3" false 0 "None"))
                  (if (Utilities|IsValid (.HitActor (Collision|BreakHitResult _outhit_2)))
                    (if (not (Actor|ActorHasTag (.HitActor (Collision|BreakHitResult _outhit_2)) "Death"))
                      (if (.bBlockingHit (Collision|BreakHitResult _outhit_2)) :!label _label_4
                        (Transformation|SetActorLocation (+ (.Location (Collision|BreakHitResult _outhit_2)) "0, 0,100.000000") false false)
                        (goto _label_3)))
                    (else
                      (goto _label_4))))))
            (else
              (goto _label_2))))
        (:CYCLONE
          ;[1 1 1] Cyclone
          (Game|SpawnActorfromClass "/Game/Blueprints/Spells/CycloneSpell_BP.CycloneSpell_BP_C" (Math|Transform|MakeTransform (+ (Transformation|GetWorldLocation _bottomspellposition) "0, 0,2500.000000") (Transformation|GetWorldRotation _bottomspellposition) "3.000000,3.000000,4.600000") "Undefined" 0 self)
          (CallFunction|BroadcastCyclone))
        (:MEDITATE
          ;[1 1 1] Meditate
          (bind _returnvalue_9 (Class|CharacterBase|GetSpellRank "MEDITATE"))
          (Variables|Default|SetChannelingMeditate true)
          (CallFunction|BroadcastMeditate)
          (bind _returnvalue_10 (Class|SpellAttributes|GetDuration "MEDITATE" _returnvalue_9))
          (Utilities|FlowControl|RetriggerableDelay _returnvalue_10)
          (if (Variables|Default|GetChannelingMeditate)
            (Variables|Default|SetChannelingMeditate false)
            (CallFunction|BroadcastCancelMediate)))))))

(event Custom|ClientUseProjectingSpell
  (params (Spell :type Spells%20Enum :default "EMPTY"))
  ;[1 1 1] Projection effect
  (bind _returnvalue (Class|CharacterBase|GetSpellRank Spell))
  (bind _returnvalue_2 (Class|SpellAttributes|GetRange Spell _returnvalue))
  (bind _returnvalue_3 (Class|CharacterBase|GetAimLocation _returnvalue_2 true))
  (bind _returnvalue_4 (Game|SpawnActorfromClass "/Game/Blueprints/Spells/ProjectingSpell_BP.ProjectingSpell_BP_C" (Math|Transform|MakeTransform _returnvalue_3) "Undefined" self 0))
  (Variables|Default|SetProjectingSpell _returnvalue_4)
  (Default|ToggleCrosshair (Variables|Default|GetBaseUI) false)
  (Default|InitializeProjectingSpell _returnvalue_4 Spell _returnvalue))

(event Custom|BroadcastPlayAnimation
  (params (Spell :type Spells%20Enum :default "EMPTY"))
  ;[1 1 1] Projection spell activation
)

(event Custom|ClientActivateProjectionSpell
  ;[1 1 1] Projection spell activation
  (Default|ToggleCrosshair (Variables|Default|GetBaseUI) true))

(event EventActivateProjectionSpellBP
  (params (spell :type Spells%20Enum :default "EMPTY") (location :type Vector :default "0, 0, 0"))
  (bind _returnvalue (Math|Transform|MakeTransform location))
  ;[1 1 1] Projection spell activation
  (CallFunction|ClientActivateProjectionSpell)
  (CallFunction|BroadcastPlayAnimation spell)
  (switch Utilities|FlowControl|Switch|SwitchonSpells spell
    (:FLAMESTRIKE
      ;[1 1 1] Flamestrike
      (Game|SpawnActorfromClass "/Game/Blueprints/Spells/FlamestrikeSpell_BP.FlamestrikeSpell_BP_C" _returnvalue "Undefined" 0 self))
    (:CONTAINMENT_FENCE
      ;[1 1 1] Containment Fence
      (Game|SpawnActorfromClass "/Game/Blueprints/Spells/ContainmentFenceSpell_BP.ContainmentFenceSpell_BP_C" _returnvalue "Undefined" 0 self))))

(event EventCancelProjectionSpellBP
  (bind _projectingspell (Variables|Default|GetProjectingSpell))
  ;[1 1 1] Cancel projection
  (if (Utilities|IsValid _projectingspell)
    (Actor|DestroyActor _projectingspell)
    (Default|ToggleCrosshair (Variables|Default|GetBaseUI) true)))

(fn ConstructionScript)