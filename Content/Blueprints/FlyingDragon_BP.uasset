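; Flying dragon character that roams the sky at a fixed altitude between random points in a large rectangular area.
; On BeginPlay it sets the flying flag on its mountain dragon animation Blueprint, and the server places it at a random start point.
; Each server tick drives velocity along its forward vector while smoothly turning toward the destination.
; Nearing the destination picks a new random point and random speed.
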(event Custom|FindNewDestination
  (Variables|Default|SetDestination (Math|Vector|MakeVector (Math|Random|RandomFloatinRange 0.0 6.8e+04) (Math|Random|RandomFloatinRange 0.0 1e+05) 2e+04))
  (Variables|Default|SetSpeed (Math|Random|RandomFloatinRange 1e+03 5e+03)))

(event EventBeginPlay
  (bind _asmountain_dragon_animation_blueprint (Utilities|Casting|CastToMountainDragon_AnimationBlueprint (Components|SkeletalMesh|GetAnimInstance (Variables|Character|GetMesh))))
  (Variables|/Game/Characters/QuadrapedCreatures/MountainDragon/Custom/MountainDragon_AnimationBlueprint.MountainDragon_AnimationBlueprint_C|SetisFlying _asmountain_dragon_animation_blueprint true)
  (if (Networking|IsServer)
    (Transformation|SetActorLocation (Math|Vector|MakeVector (Math|Random|RandomFloatinRange 0.0 6.8e+04) (Math|Random|RandomFloatinRange 0.0 1e+05) 2e+04) false false)
    (CallFunction|FindNewDestination)))

(event EventTick
  (params (DeltaSeconds :type Float%20%28single-precision%29))
  (if (Networking|IsServer)
    (Variables|/Script/Engine.MovementComponent|SetVelocity (Variables|Character|GetCharacterMovement) (* (Transformation|GetActorForwardVector) (Variables|Default|GetSpeed)))
    (Transformation|SetActorRotation (Math|Interpolation|RInterpTo (Transformation|GetActorRotation) (Math|Conversions|RotationFromXVector (- (Variables|Default|GetDestination) (Transformation|GetActorLocation))) DeltaSeconds 0.5))
    (if (<= (Math|Vector|VectorLength (- (Variables|Default|GetDestination) (Transformation|GetActorLocation))) 1e+04)
      (CallFunction|FindNewDestination))))

(fn ConstructionScript)