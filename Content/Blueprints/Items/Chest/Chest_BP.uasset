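; Loot chest actor that opens when a CharacterBase overlaps its collider on the server, then spawns random items.
; A timeline replays to swing three lock pivots open in sequence, advancing a Lock counter, before a second timeline raises the lid.
; Once the lid finishes, the server spawns one to three RandomItem_BP actors at fixed spawn points.
; A close event resets the lock rotations, but its call is unconnected.
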(event OnComponentBeginOverlap(Collider)
  (params (OverlappedComponent :type Primitive%20Component%20Object%20Reference) (OtherActor :type Actor%20Object%20Reference) (OtherComp :type Primitive%20Component%20Object%20Reference) (OtherBodyIndex :type Integer) (bFromSweep :type Boolean) (SweepResult :type Hit%20Result%20Structure%20%28by%20ref%29))
  (if (Networking|IsServer)
    (if (== (Variables|Default|GetLock) 0)
      (if (Utilities|ClassIsChildOf (Utilities|GetClass OtherActor) "/Script/ExilesOfEternity.CharacterBase")
        (CallFunction|OpenChest)))))

(event Custom|Close_Chest
  ;[1 1 1] Close Locks
  (Utilities|FlowControl|Sequence
    (:then_0
      ;[1 1 1] Open Locks
      (bind _lerp (Timeline|Timeline_0 Stop)
        (:Update
          (Transformation|SetRelativeRotation (Utilities|Select :Index (Variables|Default|GetLock) :Option%200 (Variables|Default|GetLockPivot01) :Option%201 (Variables|Default|GetLockPivot02) :Option%202 (Variables|Default|GetLockPivot03)) (Math|Rotator|MakeRotator 0.0 (Math|Float|Lerp 0.0 -1.8e+02 _lerp) 9e+01) false false))
        (:Finished
          (Variables|Default|SetLock (+ (Variables|Default|GetLock) 1))
          (Utilities|FlowControl|Delay 0.0)
          (if (>= (Variables|Default|GetLock) 3)
            ;[1 1 1] Open_Lid
            (bind _lerp_2 (Timeline|OpenChest PlayFromStart)
              (:Update
                (Transformation|SetRelativeRotation (Variables|Default|GetChest_Base_Chest_Top) (Math|Rotator|MakeRotator (Math|Float|Lerp 0.0 1.5e+02 _lerp_2) 0.0 1.8e+02) false false))
              (:Finished
                (if (Networking|IsServer)
                  (for _index (range 0 (Math|Random|RandomIntegerinRange 0 2))
                    (switch int _index
                      (:0
                        (Game|SpawnActorfromClass "/Game/Blueprints/Items/RandomItem_BP.RandomItem_BP_C" (Math|Transform|MakeTransform (Transformation|GetWorldLocation (Variables|Default|GetSpawnPostion2))) "AlwaysSpawn" 0 0))
                      (:1
                        (Game|SpawnActorfromClass "/Game/Blueprints/Items/RandomItem_BP.RandomItem_BP_C" (Math|Transform|MakeTransform (Transformation|GetWorldLocation (Variables|Default|GetSpawnPostion1))) "AlwaysSpawn" 0 0))
                      (:2
                        (Game|SpawnActorfromClass "/Game/Blueprints/Items/RandomItem_BP.RandomItem_BP_C" (Math|Transform|MakeTransform (Transformation|GetWorldLocation (Variables|Default|GetSpawnPostion3))) "AlwaysSpawn" 0 0)))))))
            (else
              (Timeline|Timeline_0 PlayFromStart))))))
    (:then_1
      (Transformation|SetRelativeRotation (Variables|Default|GetLockPivot01) "0,90.000000, 0" false false))))

(event Custom|Open_Chest
  ;[1 1 1] Open Locks
  (if (>= (Variables|Default|GetLock) 3) :!label _label
    ;[1 1 1] Open_Lid
    (bind _lerp (Timeline|OpenChest PlayFromStart)
      (:Update
        (Transformation|SetRelativeRotation (Variables|Default|GetChest_Base_Chest_Top) (Math|Rotator|MakeRotator (Math|Float|Lerp 0.0 1.5e+02 _lerp) 0.0 1.8e+02) false false))
      (:Finished
        (if (Networking|IsServer)
          (for _index (range 0 (Math|Random|RandomIntegerinRange 0 2))
            (switch int _index
              (:0
                (Game|SpawnActorfromClass "/Game/Blueprints/Items/RandomItem_BP.RandomItem_BP_C" (Math|Transform|MakeTransform (Transformation|GetWorldLocation (Variables|Default|GetSpawnPostion2))) "AlwaysSpawn" 0 0))
              (:1
                (Game|SpawnActorfromClass "/Game/Blueprints/Items/RandomItem_BP.RandomItem_BP_C" (Math|Transform|MakeTransform (Transformation|GetWorldLocation (Variables|Default|GetSpawnPostion1))) "AlwaysSpawn" 0 0))
              (:2
                (Game|SpawnActorfromClass "/Game/Blueprints/Items/RandomItem_BP.RandomItem_BP_C" (Math|Transform|MakeTransform (Transformation|GetWorldLocation (Variables|Default|GetSpawnPostion3))) "AlwaysSpawn" 0 0)))))))
    (else
      (bind _lerp_2 (Timeline|Timeline_0 PlayFromStart)
        (:Update
          (Transformation|SetRelativeRotation (Utilities|Select :Index (Variables|Default|GetLock) :Option%200 (Variables|Default|GetLockPivot01) :Option%201 (Variables|Default|GetLockPivot02) :Option%202 (Variables|Default|GetLockPivot03)) (Math|Rotator|MakeRotator 0.0 (Math|Float|Lerp 0.0 -1.8e+02 _lerp_2) 9e+01) false false))
        (:Finished
          (Variables|Default|SetLock (+ (Variables|Default|GetLock) 1))
          (Utilities|FlowControl|Delay 0.0)
          (goto _label))))))

(event EventBeginPlay)

(fn ConstructionScript)