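; ItemBase_BP is a base actor for world items that characters can pick up.
; On the server, BeginPlay enables pickup after a one-second delay.
; PickUpItem runs server-only, adds the Item to a CharacterBase's inventory, and on success sends a pickup message to its PlayerControllerBase, triggers a client pickup sound and destroys the actor.
; The overlap event is empty, so pickup relies on an external call.
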(event Custom|PickUpItem
  (params (PlayerCharacter :type Character%20Base%20BP%20Object%20Reference))
  (if (Networking|IsServer)
    (if (Variables|Default|GetCanBePickedUp)
      (if (Utilities|ClassIsChildOf (Utilities|GetClass PlayerCharacter) "/Script/ExilesOfEternity.CharacterBase")
        (bind _returnvalue (Class|CharacterBase|AddItem PlayerCharacter (Variables|Default|GetItem)))
        (if _returnvalue
          (bind _asplayer_controller_base (Utilities|Casting|CastToPlayerControllerBase (Pawn|GetController PlayerCharacter)))
          (bind _returnvalue_2 (Class|SpellAttributes|GetItemName (Variables|Default|GetItem)))
          (Class|PlayerControllerBase|AddMessage _asplayer_controller_base (Utilities|String|Append "You picked up a " _returnvalue_2) false)
          (Default|ClientPickUpItemSound PlayerCharacter)
          (Actor|DestroyActor))))))

(event EventBeginPlay
  (if (Networking|IsServer)
    (Utilities|FlowControl|Delay 1.0)
    (Variables|Default|SetCanBePickedUp true)))

(event Collision|EventActorBeginOverlap
  (params (OtherActor :type Actor%20Object%20Reference)))

(fn ConstructionScript)