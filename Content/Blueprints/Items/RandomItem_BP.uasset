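; Random item placeholder that becomes one of several pickups, such as potions, a rune or a stone, when play begins.
; On the server, BeginPlay rolls a random integer and spawns the matching item at the placeholder's location and rotation, ignoring collisions, then destroys the placeholder.
; One of the five equally weighted branches has no class set on its spawn.
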(event EventBeginPlay
  (bind _returnvalue (Transformation|GetActorLocation))
  (bind _returnvalue_2 (Transformation|GetActorRotation))
  (bind _returnvalue_3 (Math|Transform|MakeTransform _returnvalue _returnvalue_2))
  (if (Networking|IsServer)
    (switch int (Math|Random|RandomIntegerinRange 1 5)
      (:1
        (Game|SpawnActorfromClass "/Game/Blueprints/Items/HealthPotion_BP.HealthPotion_BP_C" _returnvalue_3 "AlwaysSpawn" 0 0))
      (:2
        (Game|SpawnActorfromClass "/Game/Blueprints/Items/RechargePotion_BP.RechargePotion_BP_C" _returnvalue_3 "AlwaysSpawn" 0 0))
      (:3
        (Game|SpawnActorfromClass "/Game/Blueprints/Items/LaunchRune_BP.LaunchRune_BP_C" _returnvalue_3 "AlwaysSpawn" 0 0))
      (:4
        (Game|SpawnActorfromClass "/Game/Blueprints/Items/TeleportationRune_BP.TeleportationRune_BP_C" _returnvalue_3 "AlwaysSpawn" 0 0))
      (:5
        (Game|SpawnActorfromClass "/Game/Blueprints/Items/ConstitutionStone_BP.ConstitutionStone_BP_C" _returnvalue_3 "AlwaysSpawn" 0 0)))
    (Actor|DestroyActor)))

(fn ConstructionScript
  (|CallParentFunction))