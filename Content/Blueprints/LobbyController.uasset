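; LobbyController is a lobby Blueprint that shows either the Serath or the Gideon character according to the saved character choice.
; It loads the "Settings" save slot as Settings_BP, creating a new object if that fails, then toggles both root components' visibility by CharacterName, with Gideon as the fallback.
; Marked as a temporary solution, it repeats the whole load and toggle on every Tick as well as at BeginPlay.
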(event EventTick
  (params (DeltaSeconds :type Float%20%28single-precision%29))
  ;[1 1 1] Temp solution
  (bind _returnvalue (SaveGame|LoadGamefromSlot "Settings"))
  (bind _assettings_bp (Utilities|Casting|CastToSettings_BP _returnvalue)
    (:then
      (Variables|Default|SetSettings _assettings_bp))
    (:CastFailed
      (bind _returnvalue_2 (SaveGame|CreateSaveGameObject "/Game/Blueprints/Settings_BP.Settings_BP_C"))
      (Variables|Default|SetSettings _returnvalue_2)))
  (if (Utilities|Enum|Equal(Enum) (Variables|/Game/Blueprints/Settings_BP.Settings_BP_C|GetCharacterName (Variables|Default|GetSettings)) "Serath")
    (if true
      (Rendering|SetVisibility (Variables|/Script/Engine.Actor|GetRootComponent (Variables|Default|GetSerath)) true false)
      (Rendering|SetVisibility (Variables|/Script/Engine.Actor|GetRootComponent (Variables|Default|GetGideon)) false false))
    (else
      (Rendering|SetVisibility (Variables|/Script/Engine.Actor|GetRootComponent (Variables|Default|GetSerath)) false false)
      (Rendering|SetVisibility (Variables|/Script/Engine.Actor|GetRootComponent (Variables|Default|GetGideon)) true false))))

(event EventBeginPlay
  ;[1 1 1] Temp solution
  (bind _returnvalue (SaveGame|LoadGamefromSlot "Settings"))
  (bind _assettings_bp (Utilities|Casting|CastToSettings_BP _returnvalue)
    (:then
      (Variables|Default|SetSettings _assettings_bp))
    (:CastFailed
      (bind _returnvalue_2 (SaveGame|CreateSaveGameObject "/Game/Blueprints/Settings_BP.Settings_BP_C"))
      (Variables|Default|SetSettings _returnvalue_2)))
  (if (Utilities|Enum|Equal(Enum) (Variables|/Game/Blueprints/Settings_BP.Settings_BP_C|GetCharacterName (Variables|Default|GetSettings)) "Serath")
    (if true
      (Rendering|SetVisibility (Variables|/Script/Engine.Actor|GetRootComponent (Variables|Default|GetSerath)) true false)
      (Rendering|SetVisibility (Variables|/Script/Engine.Actor|GetRootComponent (Variables|Default|GetGideon)) false false))
    (else
      (Rendering|SetVisibility (Variables|/Script/Engine.Actor|GetRootComponent (Variables|Default|GetSerath)) false false)
      (Rendering|SetVisibility (Variables|/Script/Engine.Actor|GetRootComponent (Variables|Default|GetGideon)) true false))))

(fn ConstructionScript)