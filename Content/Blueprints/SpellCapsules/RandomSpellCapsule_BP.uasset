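; Random spell capsule placeholder that swaps itself for one of several spell capsule pickups when play begins.
; On the server, BeginPlay rolls one of eight equally likely cases, spawns that capsule at its own location and rotation, then destroys itself.
; Six cases map to Flamestrike, Shield, ContainmentFence, Cyclone, Meditate and Frostbolt capsules.
; The other two spawn calls have no class set.
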(event EventBeginPlay
  (bind _returnvalue (Transformation|GetActorLocation))
  (bind _returnvalue_2 (Transformation|GetActorRotation))
  (bind _returnvalue_3 (Math|Transform|MakeTransform _returnvalue _returnvalue_2))
  (if (Networking|IsServer)
    (switch int (Math|Random|RandomIntegerinRange 1 8)
      (:1
        (Game|SpawnActorfromClass "/Game/Blueprints/SpellCapsules/FlamestrikeCapsule_BP.FlamestrikeCapsule_BP_C" _returnvalue_3 "AlwaysSpawn" 0 0))
      (:2
        (Game|SpawnActorfromClass "/Game/Blueprints/SpellCapsules/ShieldCapsule_BP.ShieldCapsule_BP_C" _returnvalue_3 "AlwaysSpawn" 0 0))
      (:3
        (Game|SpawnActorfromClass "/Game/Blueprints/SpellCapsules/BlinkCapsule_BP.BlinkCapsule_BP_C" _returnvalue_3 "AlwaysSpawn" 0 0))
      (:4
        (Game|SpawnActorfromClass "/Game/Blueprints/SpellCapsules/ContainmentFenceCapsule_BP.ContainmentFenceCapsule_BP_C" _returnvalue_3 "AlwaysSpawn" 0 0))
      (:5
        (Game|SpawnActorfromClass "/Game/Blueprints/SpellCapsules/CycloneCapsule_BP.CycloneCapsule_BP_C" _returnvalue_3 "AlwaysSpawn" 0 0))
      (:6
        (Game|SpawnActorfromClass "/Game/Blueprints/SpellCapsules/MeditateCapsule_BP.MeditateCapsule_BP_C" _returnvalue_3 "AlwaysSpawn" 0 0))
      (:7
        (Game|SpawnActorfromClass "/Game/Blueprints/SpellCapsules/FrostboltCapsule_BP.FrostboltCapsule_BP_C" _returnvalue_3 "AlwaysSpawn" 0 0))
      (:8
        (Game|SpawnActorfromClass "/Game/Blueprints/SpellCapsules/GlacialForceCapsule_BP.GlacialForceCapsule_BP_C" _returnvalue_3 "AlwaysSpawn" 0 0)))
    (Actor|DestroyActor)))

(fn ConstructionScript
  (|CallParentFunction))