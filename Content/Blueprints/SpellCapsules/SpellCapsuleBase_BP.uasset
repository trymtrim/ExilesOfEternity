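; Base spell capsule pickup that grants its spell and rank to a character that overlaps it.
; On initialization, the server takes the rank from the owning character and enables pickup after a short delay, while clients tint the particles and cylinder and apply the spell's icon through a dynamic material.
; Overlaps are server-authoritative: a successful spell add messages the player's controller, notifies the client and destroys the capsule.
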(event Custom|InitializeCapsule
  (bind _cylinder (Variables|Default|GetCylinder))
  (if (Networking|IsServer)
    (bind _ascharacter_base (Utilities|Casting|CastToCharacterBase (Components|GetOwner))
      (:then
        (bind _returnvalue (Class|CharacterBase|GetSpellRank _ascharacter_base (Variables|Default|GetSpell)))
        (Variables|Default|SetRank _returnvalue))
      (:CastFailed
        _))
    (Utilities|FlowControl|Delay 1.0)
    (Variables|Default|SetCanBePickedUp true)
    (else
      (bind _returnvalue_2 (Class|SpellAttributes|GetIconColor (Variables|Default|GetSpell)))
      (Effects|Components|ParticleSystem|SetVectorParameter (Variables|Default|GetParticleSystem) "Color" (Math|Conversions|ToVector(LinearColor) (Math|Conversions|ToLinearColor(Color) _returnvalue_2)))
      (bind _returnvalue_3 (Rendering|Material|CreateDynamicMaterialInstance _cylinder 0 "/Game/Shaders/SpellCapsules/SpellCapsules_M_Inst.SpellCapsules_M_Inst" "" :!class /Script/Engine.PrimitiveComponent))
      (bind _returnvalue_4 (Class|SpellAttributes|GetIcon (Variables|Default|GetSpell)))
      (Rendering|Material|SetTextureParameterValue _returnvalue_3 "Icon" _returnvalue_4)
      (Rendering|Material|SetVectorParameterValueonMaterials _cylinder "Color" (Math|Conversions|ToVector(LinearColor) (Math|Conversions|ToLinearColor(Color) _returnvalue_2))))))

(event EventBeginPlay
  (bind _cylinder (Variables|Default|GetCylinder))
  (if (Networking|IsServer)
    (bind _ascharacter_base (Utilities|Casting|CastToCharacterBase (Components|GetOwner))
      (:then
        (bind _returnvalue (Class|CharacterBase|GetSpellRank _ascharacter_base (Variables|Default|GetSpell)))
        (Variables|Default|SetRank _returnvalue))
      (:CastFailed
        _))
    (Utilities|FlowControl|Delay 1.0)
    (Variables|Default|SetCanBePickedUp true)
    (else
      (bind _returnvalue_2 (Class|SpellAttributes|GetIconColor (Variables|Default|GetSpell)))
      (Effects|Components|ParticleSystem|SetVectorParameter (Variables|Default|GetParticleSystem) "Color" (Math|Conversions|ToVector(LinearColor) (Math|Conversions|ToLinearColor(Color) _returnvalue_2)))
      (bind _returnvalue_3 (Rendering|Material|CreateDynamicMaterialInstance _cylinder 0 "/Game/Shaders/SpellCapsules/SpellCapsules_M_Inst.SpellCapsules_M_Inst" "" :!class /Script/Engine.PrimitiveComponent))
      (bind _returnvalue_4 (Class|SpellAttributes|GetIcon (Variables|Default|GetSpell)))
      (Rendering|Material|SetTextureParameterValue _returnvalue_3 "Icon" _returnvalue_4)
      (Rendering|Material|SetVectorParameterValueonMaterials _cylinder "Color" (Math|Conversions|ToVector(LinearColor) (Math|Conversions|ToLinearColor(Color) _returnvalue_2))))))

(event Collision|EventActorBeginOverlap
  (params (OtherActor :type Actor%20Object%20Reference))
  (if (Networking|IsServer)
    (if (Variables|Default|GetCanBePickedUp)
      (if (Utilities|ClassIsChildOf (Utilities|GetClass OtherActor) "/Script/ExilesOfEternity.CharacterBase")
        (bind _ascharacter_base_bp (Utilities|Casting|CastToCharacterBase_BP OtherActor))
        (bind _returnvalue (Class|CharacterBase|AddSpell _ascharacter_base_bp (Variables|Default|GetSpell) (Variables|Default|GetRank) false))
        (if _returnvalue
          (bind _asplayer_controller_base (Utilities|Casting|CastToPlayerControllerBase (Pawn|GetController _ascharacter_base_bp)))
          (bind _returnvalue_2 (Class|SpellAttributes|GetName (Variables|Default|GetSpell)))
          (Class|PlayerControllerBase|AddMessage _asplayer_controller_base (Utilities|String|Append "You unlocked " _returnvalue_2) false)
          (Default|ClientSpellPickUp _ascharacter_base_bp)
          (Actor|DestroyActor))))))

(fn ConstructionScript)