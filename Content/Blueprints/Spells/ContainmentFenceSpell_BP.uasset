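; Containment Fence spell actor that shows a force field sized and timed by the instigating character's spell rank.
; On spawn it scales horizontally to the rank's radius and passes that size to the fence material's mask.
; A timeline animates the material's opacity and mask height.
; The server destroys the actor when the duration ends, while clients play a delayed looping-phase sound and fade it out just before expiry.
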(event EventBeginPlay
  (bind _containmentfence (Variables|Default|GetContainmentFence))
  (Utilities|FlowControl|Sequence
    (:then_0
      (bind _ascharacter_base (Utilities|Casting|CastToCharacterBase (Variables|Actor|GetInstigator)))
      (bind _returnvalue (Class|CharacterBase|GetSpellRank _ascharacter_base "CONTAINMENT_FENCE"))
      (bind _returnvalue_2 (Class|SpellAttributes|GetRadius "CONTAINMENT_FENCE" _returnvalue))
      (Transformation|SetActorScale3D (Math|Vector|MakeVector (/ _returnvalue_2 5e+02) (/ _returnvalue_2 5e+02) 1.0))
      (if (Networking|IsServer)
        (bind _returnvalue_3 (Class|SpellAttributes|GetDuration "CONTAINMENT_FENCE" _returnvalue))
        (Utilities|FlowControl|Delay _returnvalue_3)
        (Actor|DestroyActor)
        (else
          (bind _returnvalue_4 (Class|SpellAttributes|GetDuration "CONTAINMENT_FENCE" _returnvalue))
          (Utilities|FlowControl|Delay (- _returnvalue_4 0.3))
          (if (Utilities|IsValid (stale _returnvalue_5))
            (Audio|Components|Audio|FadeOut (stale _returnvalue_5) 0.3 0.0 :!class /Script/Engine.AudioComponent)))))
    (:then_1
      (Rendering|Material|SetScalarParameterValueonMaterials _containmentfence "MaskSize" (* _returnvalue_2 2.0))
      (if (not (Networking|IsServer))
        (Utilities|FlowControl|Delay 0.5)
        (bind _returnvalue_5 (Audio|SpawnSoundAttached "/Game/Audio/Spells/ContainmentFence/ContainmentFence_WhileActive.ContainmentFence_WhileActive" (Variables|Default|GetAudio) "None" "0, 0, 0" "0, 0, 0" "KeepRelativeOffset" true 1.0 1.0 0.0 0 0))))
    (:then_2
      (bind _opacity (Timeline|ForceFieldOpacity PlayFromStart)
        (:Update
          (Rendering|Material|SetScalarParameterValueonMaterials _containmentfence "Opacity" _opacity)
          (Rendering|Material|SetScalarParameterValueonMaterials _containmentfence "MaskHeight" _opacity))))))

(fn ConstructionScript)