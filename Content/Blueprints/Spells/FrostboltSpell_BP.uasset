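; Frostbolt spell projectile that bursts on impact, damaging nearby characters and slowing players.
; On BeginPlay the server loads rank-based damage, radius and duration from the caster, while clients attach the projectile particle.
; A server-side per-tick box trace or sphere overlap triggers a manual radial falloff over all players and AI, slowing only non-immune players and sparing the owning player.
; It then plays radius-scaled impact effects and destroys itself, as it also does after a short lifetime.
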(event OnComponentBeginOverlap(Sphere)
  (params (OverlappedComponent :type Primitive%20Component%20Object%20Reference) (OtherActor :type Actor%20Object%20Reference) (OtherComp :type Primitive%20Component%20Object%20Reference) (OtherBodyIndex :type Integer) (bFromSweep :type Boolean) (SweepResult :type Hit%20Result%20Structure%20%28by%20ref%29))
  (bind _damage (Variables|Default|GetDamage))
  (bind _damage_2 (Variables|Default|GetDamage))
  (bind _radius (Variables|Default|GetRadius))
  (bind _radius_2 (Variables|Default|GetRadius))
  (bind _returnvalue (/ _damage_2 5.0))
  (bind _returnvalue_2 (/ _damage 5.0))
  (if (Networking|IsServer)
    (if (!= OtherActor (Components|GetOwner))
      (Variables|Default|SetImpactPoint (.ImpactPoint (Collision|BreakHitResult SweepResult)))
      ;[1 1 1] Radial damage with falloff against players
      (bind _outactors (Actor|GetAllActorsOfClass "/Script/ExilesOfEternity.CharacterBase"))
      (for _array_element _outactors
        (if (<= (Math|Vector|VectorLength (- (Transformation|GetActorLocation _array_element) (Variables|Default|GetImpactPoint))) _radius)
          (if (!= _array_element (Components|GetOwner))
            (Game|Damage|ApplyDamage _array_element (+ (- (Variables|Default|GetDamage) (Math|Float|MapRangeClamped (Math|Vector|VectorLength (- (Transformation|GetActorLocation _array_element) (Variables|Default|GetImpactPoint))) 75.0 _radius _returnvalue_2 _damage)) _returnvalue_2) 0 (Variables|Actor|GetInstigator))
            (bind _returnvalue_3 (Class|CharacterBase|GetImmunity _array_element))
            (if (not _returnvalue_3)
              (Class|CharacterBase|SetSlowEffect _array_element (+ 1.0 (/ (Math|Conversions|ToFloat(Integer) (Variables|Default|GetRank)) 2.0)) (Variables|Default|GetDuration))))))
      ;[1 1 1] Radial damage with falloff against AI
      (bind _outactors_2 (Actor|GetAllActorsOfClass "/Script/ExilesOfEternity.AICharacterBase"))
      (for _array_element_2 _outactors_2
        (if (<= (Math|Vector|VectorLength (- (Transformation|GetActorLocation _array_element_2) (Variables|Default|GetImpactPoint))) _radius_2)
          (Game|Damage|ApplyDamage _array_element_2 (+ (- (Variables|Default|GetDamage) (Math|Float|MapRangeClamped (Math|Vector|VectorLength (- (Transformation|GetActorLocation _array_element_2) (Variables|Default|GetImpactPoint))) 75.0 _radius_2 _returnvalue _damage_2)) _returnvalue) 0 (Variables|Actor|GetInstigator))))
      (CallFunction|ImpactFX (Variables|Default|GetImpactPoint))
      (Actor|DestroyActor))))

(event Custom|ImpactFX
  (params (Location :type Vector))
  ;[1 1 1] ImpactFX
  (Effects|SpawnEmitteratLocation "/Game/FX/FXVarietyPack/Particles/P_ky_waterBallHit.P_ky_waterBallHit" Location "0, 0, 0" (Math|Conversions|ToVector(Float) (/ (Variables|Default|GetRadius) 125.0)))
  (Audio|SpawnSoundAttached "/Game/Audio/Spells/Frostbolt/Frostbolt_OnHit.Frostbolt_OnHit" (Variables|Default|GetAudio) "None" "0, 0, 0" "0, 0, 0" "KeepRelativeOffset" false 1.0 1.0 0.0 0 0))

(event EventBeginPlay
  (if (Networking|IsServer)
    (bind _ascharacter_base (Utilities|Casting|CastToCharacterBase (Variables|Actor|GetInstigator)))
    (bind _output_get (Variables|Default|SetCharacterController _ascharacter_base))
    (bind _returnvalue (Class|CharacterBase|GetSpellRank _output_get "FROSTBOLT"))
    (Variables|Default|SetRank _returnvalue)
    (bind _returnvalue_2 (Class|SpellAttributes|GetRadius "FROSTBOLT" _returnvalue))
    (bind _returnvalue_3 (Class|SpellAttributes|GetDuration "FROSTBOLT" _returnvalue))
    (bind _returnvalue_4 (Class|SpellAttributes|GetDamage "FROSTBOLT" _returnvalue))
    (Variables|Default|SetDamage _returnvalue_4)
    (Variables|Default|SetDuration _returnvalue_3)
    (Variables|Default|SetRadius _returnvalue_2)
    (Utilities|FlowControl|Delay 1.5)
    (CallFunction|ImpactFX (Transformation|GetActorLocation))
    (Actor|DestroyActor)
    (else
      (Effects|SpawnEmitterAttached "/Game/FX/FXVarietyPack/Particles/P_ky_waterBall.P_ky_waterBall" (Variables|Default|GetSphere) "None" "0, 0, 0" "90.000000,180.000000,180.000000" "15.000000,15.000000,15.000000"))))

(event EventTick
  (params (DeltaSeconds :type Float%20%28single-precision%29))
  (bind _returnvalue (Transformation|GetActorLocation))
  (bind _damage (Variables|Default|GetDamage))
  (bind _damage_2 (Variables|Default|GetDamage))
  (bind _radius (Variables|Default|GetRadius))
  (bind _radius_2 (Variables|Default|GetRadius))
  (bind _returnvalue_2 (/ _damage_2 5.0))
  (bind _returnvalue_3 (/ _damage 5.0))
  (if (Networking|IsServer)
    (bind (_outhit _returnvalue_4) (Class|KismetSystemLibrary|BoxTraceSingleforObjects _returnvalue _returnvalue "50.000000,50.000000,50.000000" (Transformation|GetActorRotation) (Utilities|Array|MakeArray "ObjectTypeQuery3") false 0 "None" true "(R=0.000000,G=1.000000,B=0.990451,A=1.000000)" "(R=0.000000,G=1.000000,B=0.000000,A=1.000000)" 2e+01))
    (if _returnvalue_4
      (if (!= (.HitActor (Collision|BreakHitResult _outhit)) (Components|GetOwner))
        (Variables|Default|SetImpactPoint (.Location (Collision|BreakHitResult _outhit)))
        ;[1 1 1] Radial damage with falloff against players
        (bind _outactors (Actor|GetAllActorsOfClass "/Script/ExilesOfEternity.CharacterBase"))
        (for _array_element _outactors
          (if (<= (Math|Vector|VectorLength (- (Transformation|GetActorLocation _array_element) (Variables|Default|GetImpactPoint))) _radius)
            (if (!= _array_element (Components|GetOwner))
              (Game|Damage|ApplyDamage _array_element (+ (- (Variables|Default|GetDamage) (Math|Float|MapRangeClamped (Math|Vector|VectorLength (- (Transformation|GetActorLocation _array_element) (Variables|Default|GetImpactPoint))) 75.0 _radius _returnvalue_3 _damage)) _returnvalue_3) 0 (Variables|Actor|GetInstigator))
              (bind _returnvalue_5 (Class|CharacterBase|GetImmunity _array_element))
              (if (not _returnvalue_5)
                (Class|CharacterBase|SetSlowEffect _array_element (+ 1.0 (/ (Math|Conversions|ToFloat(Integer) (Variables|Default|GetRank)) 2.0)) (Variables|Default|GetDuration))))))
        ;[1 1 1] Radial damage with falloff against AI
        (bind _outactors_2 (Actor|GetAllActorsOfClass "/Script/ExilesOfEternity.AICharacterBase"))
        (for _array_element_2 _outactors_2
          (if (<= (Math|Vector|VectorLength (- (Transformation|GetActorLocation _array_element_2) (Variables|Default|GetImpactPoint))) _radius_2)
            (Game|Damage|ApplyDamage _array_element_2 (+ (- (Variables|Default|GetDamage) (Math|Float|MapRangeClamped (Math|Vector|VectorLength (- (Transformation|GetActorLocation _array_element_2) (Variables|Default|GetImpactPoint))) 75.0 _radius_2 _returnvalue_2 _damage_2)) _returnvalue_2) 0 (Variables|Actor|GetInstigator))))
        (CallFunction|ImpactFX (Variables|Default|GetImpactPoint))
        (Actor|DestroyActor)))))

(fn ConstructionScript)