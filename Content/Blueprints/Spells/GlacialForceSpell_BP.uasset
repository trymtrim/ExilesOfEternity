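; Glacial Force spell actor: a short-lived, rank-scaled sphere that damages and stuns enemy characters.
; The server sizes the sphere, snaps it to traced ground every tick, then disables damage after a second and destroys it shortly after.
; Overlaps skip teammates and immune players, cancel surviving victims' spells and only damage AI; the AI launch is unwired.
; Clients spawn water-hit particles each tick while damage is active and fade the audio.
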(event OnComponentBeginOverlap(Sphere)
  (params (OverlappedComponent :type Primitive%20Component%20Object%20Reference) (OtherActor :type Actor%20Object%20Reference) (OtherComp :type Primitive%20Component%20Object%20Reference) (OtherBodyIndex :type Integer) (bFromSweep :type Boolean) (SweepResult :type Hit%20Result%20Structure%20%28by%20ref%29))
  (bind _instigator (Variables|Actor|GetInstigator))
  (if (Networking|IsServer)
    (if (Variables|Default|GetCanDamage)
      (if (not (Utilities|Array|ContainsItem (Variables|Default|GetCharactersHit) OtherActor))
        (bind _returnvalue (Class|SpellAttributes|GetDamage "GLACIAL_FORCE" (Variables|Default|GetRank)))
        (bind _ascharacter_base (Utilities|Casting|CastToCharacterBase OtherActor)
          (:then
            (bind _asplayer_state_base (Utilities|Casting|CastToPlayerStateBase (Variables|/Script/Engine.Pawn|GetPlayerState _ascharacter_base)))
            (bind _returnvalue_2 (Class|PlayerStateBase|GetTeamNumber _asplayer_state_base))
            (bind _asplayer_state_base_2 (Utilities|Casting|CastToPlayerStateBase (Variables|/Script/Engine.Pawn|GetPlayerState (Variables|Actor|GetInstigator))))
            (bind _returnvalue_3 (Class|PlayerStateBase|GetTeamNumber _asplayer_state_base_2))
            (if (!= _returnvalue_2 _returnvalue_3)
              (bind _returnvalue_4 (Class|CharacterBase|GetImmunity _ascharacter_base))
              (if (not _returnvalue_4)
                (Game|Damage|ApplyDamage OtherActor _returnvalue 0 _instigator)
                (bind _returnvalue_5 (Class|CharacterBase|GetDead _ascharacter_base))
                (if (not _returnvalue_5)
                  (Class|CharacterBase|SetStunEffect _ascharacter_base true (Variables|Default|GetDuration))
                  (Utilities|Array|Add (Variables|Default|GetCharactersHit) OtherActor)
                  (bind _ascharacter_base_bp (Utilities|Casting|CastToCharacterBase_BP _ascharacter_base))
                  (Default|CancelCurrentSpell _ascharacter_base_bp)))))
          (:CastFailed
            (bind _asaicharacter_base (Utilities|Casting|CastToAICharacterBase OtherActor))
            (Game|Damage|ApplyDamage _asaicharacter_base _returnvalue 0 _instigator)
            (Utilities|Array|Add (Variables|Default|GetCharactersHit) _asaicharacter_base)))))))

(event EventBeginPlay
  (if (Networking|IsServer)
    (bind _ascharacter_base (Utilities|Casting|CastToCharacterBase (Variables|Actor|GetInstigator)))
    (bind _returnvalue (Class|CharacterBase|GetSpellRank _ascharacter_base "GLACIAL_FORCE"))
    (bind _output_get (Variables|Default|SetRank _returnvalue))
    (bind _returnvalue_2 (Class|SpellAttributes|GetRadius "GLACIAL_FORCE" _output_get))
    (Transformation|SetWorldScale3D (Variables|Default|GetSphere) (Math|Vector|MakeVector (/ _returnvalue_2 1e+02) (/ _returnvalue_2 1e+02) (/ _returnvalue_2 1e+02)))
    (bind _returnvalue_3 (Class|SpellAttributes|GetDuration "GLACIAL_FORCE" _output_get))
    (Variables|Default|SetDuration _returnvalue_3)
    (Utilities|FlowControl|Delay 1.0)
    (Variables|Default|SetCanDamage false)
    (Utilities|FlowControl|Delay 0.5)
    (Actor|DestroyActor)
    (else
      (Utilities|FlowControl|Delay 1.0)
      (Audio|Components|Audio|FadeOut (Variables|Default|GetAudio) 0.3 0.0 :!class /Script/Engine.AudioComponent))))

(event EventTick
  (params (DeltaSeconds :type Float%20%28single-precision%29))
  (bind _returnvalue (Transformation|GetActorLocation))
  (bind _returnvalue_2 (Transformation|GetActorLocation))
  (if (Networking|IsServer)
    (bind _outhit (Collision|LineTraceByChannel _returnvalue_2 (+ _returnvalue_2 "0, 0,5000.000000") "TraceTypeQuery3" false 0 "None"))
    (if (.bBlockingHit (Collision|BreakHitResult _outhit))
      (Transformation|SetActorLocation (.ImpactPoint (Collision|BreakHitResult _outhit)) true false)
      (else
        (bind _outhit_2 (Collision|LineTraceByChannel _returnvalue (- _returnvalue "0, 0,5000.000000") "TraceTypeQuery3" false 0 "None"))
        (if (.bBlockingHit (Collision|BreakHitResult _outhit_2))
          (Transformation|SetActorLocation (.Location (Collision|BreakHitResult _outhit_2)) true false))))
    (elif (Variables|Default|GetCanDamage)
      (Effects|SpawnEmitteratLocation "/Game/FX/FXVarietyPack/Particles/P_ky_waterBallHit.P_ky_waterBallHit" (Transformation|GetActorLocation) "0, 0, 0" (Math|Conversions|ToVector(Float) (/ (.X (Math|Vector|BreakVector (Transformation|GetActorScale3D))) 3.5))))))

(fn ConstructionScript)