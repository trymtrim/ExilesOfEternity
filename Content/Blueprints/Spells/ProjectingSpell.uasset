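; ProjectingSpell is a spell actor that follows the aim location of the character that owns it.
; On BeginPlay it casts its owner to CharacterBase and sets its maximum distance from that character's currently activated spell, with only an example projecting spell defined.
; Every Tick it queries the character's GetAimLocation with that distance and moves itself there without sweeping.
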(event EventTick
  (params (DeltaSeconds :type Float%20%28single-precision%29))
  (bind _returnvalue (Class|CharacterBase|GetAimLocation (Variables|Default|GetCharacterController) (Variables|Default|GetMaxDistance) false))
  (Transformation|SetActorLocation _returnvalue false false))

(event EventBeginPlay
  (bind _ascharacter_base (Utilities|Casting|CastToCharacterBase (Components|GetOwner)))
  (Variables|Default|SetCharacterController _ascharacter_base)
  (switch Utilities|FlowControl|Switch|SwitchonSpells (Variables|/Script/ExilesOfEternity.CharacterBase|Get_currentlyActivatedSpell (Variables|Default|GetCharacterController))
    (:EXAMPLE_PROJECTING_SPELL
      (Variables|Default|SetMaxDistance 2e+03))))

(fn ConstructionScript)