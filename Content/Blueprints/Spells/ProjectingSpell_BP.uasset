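; ProjectingSpell_BP is a spell targeting marker actor that projects a decal at the owning character's aim point.
; On BeginPlay it caches its owner as a CharacterBase, then each Tick moves itself to that character's aim location, capped at a maximum distance.
; InitializeProjectingSpell sets that distance from the spell's range and picks the decal material per spell, with only an example stun entry so far.
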(event EventTick
  (params (DeltaSeconds :type Float%20%28single-precision%29))
  (bind _returnvalue (Class|CharacterBase|GetAimLocation (Variables|Default|GetCharacterController) (Variables|Default|GetMaxDistance) false))
  (Transformation|SetActorLocation _returnvalue false false))

(event EventBeginPlay
  (bind _ascharacter_base (Utilities|Casting|CastToCharacterBase (Components|GetOwner)))
  (Variables|Default|SetCharacterController _ascharacter_base))

(fn ConstructionScript)

(fn InitializeProjectingSpell
  (params (Spell :type Spells%20Enum :default "DEFAULT_SPELL"))
  (bind _returnvalue (Class|SpellAttributes|GetRange Spell))
  (Variables|Default|SetMaxDistance _returnvalue)
  ;[1 1 1] Set decal material based on spell
  (switch Utilities|FlowControl|Switch|SwitchonSpells Spell
    (:EXAMPLE_PROJECTING_SPELL
      (Rendering|Components|Decal|SetDecalMaterial (Variables|Default|GetDecal) "/Game/FX/Spells/Stun/Stun_Decal.Stun_Decal"))))