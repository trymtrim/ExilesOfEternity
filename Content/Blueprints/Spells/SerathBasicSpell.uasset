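; Basic spell actor for Serath that damages the first valid actor overlapping its sphere.
; The server alone handles both lifetime and hits, destroying the spell one second after BeginPlay if nothing is hit sooner.
; A valid overlap with an actor other than the owner applies fixed damage, with the spell as damage causer, and destroys it immediately.
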(event OnComponentBeginOverlap(Sphere)
  (params (OverlappedComponent :type Primitive%20Component%20Object%20Reference) (OtherActor :type Actor%20Object%20Reference) (OtherComp :type Primitive%20Component%20Object%20Reference) (OtherBodyIndex :type Integer) (bFromSweep :type Boolean) (SweepResult :type Hit%20Result%20Structure%20%28by%20ref%29))
  (if (Networking|IsServer)
    (if (!= OtherActor 0)
      (if (!= OtherActor (Components|GetOwner))
        (Game|Damage|ApplyDamage OtherActor 2e+01 0 self)
        (Actor|DestroyActor)))))

(event EventBeginPlay
  (if (Networking|IsServer)
    (Utilities|FlowControl|Delay 1.0)
    (Actor|DestroyActor)))

(fn ConstructionScript)