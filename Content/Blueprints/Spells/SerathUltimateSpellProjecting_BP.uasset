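; Projection actor for Serath's ultimate spell that, while active, follows where the owning character aims, likely as a targeting preview.
; On BeginPlay it caches its parent actor as the CharacterBase to query.
; Each active Tick it moves to that character's range-limited aim location.
; If that location's vector length is huge, it instead traces straight down from the character and snaps to any blocking hit.
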(event EventTick
  (params (DeltaSeconds :type Float%20%28single-precision%29))
  (bind _charactercontroller (Variables|Default|GetCharacterController))
  (bind _returnvalue (Transformation|GetActorLocation _charactercontroller))
  (if (Variables|Default|GetIsActive)
    (bind _returnvalue_2 (Class|CharacterBase|GetAimLocation (Variables|Default|GetCharacterController) (Variables|Default|GetMaxDistance) false))
    (if (< (Math|Vector|VectorLength _returnvalue_2) 999999.0)
      (Transformation|SetActorLocation _returnvalue_2 false false)
      (else
        (bind _outhit (Collision|LineTraceByChannel _returnvalue (- _returnvalue "0, 0,50000.000000") "TraceTypeQuery3" false 0 "None"))
        (if (.bBlockingHit (Collision|BreakHitResult _outhit))
          (Transformation|SetActorLocation (.ImpactPoint (Collision|BreakHitResult _outhit)) false false))))))

(event EventBeginPlay
  (bind _ascharacter_base (Utilities|Casting|CastToCharacterBase (Actor|GetParentActor)))
  (Variables|Default|SetCharacterController _ascharacter_base))

(fn ConstructionScript)