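; Serath's ultimate spell actor, which deals random radial damage where its sphere first overlaps another actor.
; On the server, an overlap applies the damage, calls ImpactFX and destroys the actor.
; The overlap filter compares the other actor to that actor's own owner, not the spell's.
; Without a hit it calls ImpactFX and self-destructs after a timeout; ImpactFX spawns the emitter and hit sound.
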(event OnComponentBeginOverlap(Sphere)
  (params (OverlappedComponent :type Primitive%20Component%20Object%20Reference) (OtherActor :type Actor%20Object%20Reference) (OtherComp :type Primitive%20Component%20Object%20Reference) (OtherBodyIndex :type Integer) (bFromSweep :type Boolean) (SweepResult :type Hit%20Result%20Structure%20%28by%20ref%29))
  (bind _impactpoint (Collision|BreakHitResult SweepResult))
  (if (Networking|IsServer)
    (if (!= OtherActor (Components|GetOwner OtherActor))
      (Game|Damage|ApplyRadialDamage (Math|Random|RandomFloatinRange 6.0 13.0) _impactpoint 4e+02 0 0 (Variables|Actor|GetInstigator) 0 false "ECC_GameTraceChannel2")
      (CallFunction|ImpactFX _impactpoint)
      (Actor|DestroyActor))))

(event Custom|ImpactFX
  (params (Location :type Vector))
  (Effects|SpawnEmitteratLocation "/Game/FX/Spells/BaseAttack/BaseAttackFX_02.BaseAttackFX_02" Location "0, 0, 0" "1.000000,1.000000,1.000000" false)
  (Audio|SpawnSoundAttached "/Game/Audio/Spells/SerathBasicSpell/SerathBasicSpell_OnHit.SerathBasicSpell_OnHit" (Variables|Default|GetAudio) "None" "0, 0, 0" "0, 0, 0" "KeepRelativeOffset" false 1.0 1.0 0.0 0 0))

(event EventBeginPlay
  (if (Networking|IsServer)
    (Utilities|FlowControl|Delay 1e+01)
    (CallFunction|ImpactFX (Transformation|GetActorLocation))
    (Actor|DestroyActor)))

(fn ConstructionScript)